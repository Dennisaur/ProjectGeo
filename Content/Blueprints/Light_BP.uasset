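; Light actor that is lit only while the orb is in use and the player character has energy left.
; Every Tick it reads the using-orb state from PGIndicatorC and the current energy from the ProjectGeoCharacter of player 0.
; It then sets the LightComponent's visibility, propagated to its children, to match that condition.
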(event `self.ReceiveTick`
  (params (DeltaSeconds :type "Float (single-precision)"))
  (bind _lightcomponent (`self.LightComponent`))
  (if (and (`Indicator.GetUsingOrb` (`self.PG_Indicator_C`)) (> (`ProjectGeoCharacter.GetCurrentEnergy` (cast `ProjectGeoCharacter` (`GameplayStatics.GetPlayerCharacter` 0) :!pure true)) 0.0))
    (`SceneComponent.SetVisibility` _lightcomponent true true)
    (else
      (`SceneComponent.SetVisibility` _lightcomponent false true))))

(fn `UserConstructionScript`)