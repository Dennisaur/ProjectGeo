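; Door Blueprint that raises its door once a linked PGIndicatorC reports a completed charge, with no logic to close it.
; The construction script caches the door's world location as the down position and derives the up position from a Z offset scaled by door height scale.
; Tick polls the charge and plays the DoorMove timeline, whose track feeds VInterpTo's DeltaTime from the fixed start, effectively acting as a lerp alpha.
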(event `self.ReceiveTick`
  (params (DeltaSeconds :type "Float (single-precision)"))
  (if (`Indicator.GetCompletedCharge` (`self.PG_Indicator_C`))
    (bind (_direction _newtrack_0) (`Timeline|Door Move`)
      (:`Update`
        (`SceneComponent.K2_SetWorldLocation` (`self.Door`) (`KismetMathLibrary.VInterpTo` (`self.DoorDown`) (`self.DoorUp`) _newtrack_0 1.0) false false)))))

(fn `UserConstructionScript`
  (bind _output_get (set `self.DoorDown` (`SceneComponent.K2_GetComponentLocation` (`self.Door`))))
  (set `self.DoorUp` (`KismetMathLibrary.MakeVector` (.x _output_get) (.y _output_get) (+ (.z _output_get) (* 400.0 (.z (`SceneComponent.K2_GetComponentScale` (`self.Door`))))))))